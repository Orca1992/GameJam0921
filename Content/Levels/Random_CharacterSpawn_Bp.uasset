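; A spawner actor that shows a random NPC through its ChildActor component.
; From BeginPlay it loops, setting the child actor class, applying a random yaw to itself, then waiting a random 10 to 20 seconds.
; The class Select has five level NPC options, but the random index range only reaches the Level 1 and Level 2 entries.
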(event EventBeginPlay
  ;[1 1 1] Random Actor Spawn
  (ChildActorComponent|SetChildActorClass (Variables|Default|GetChildActor) (Utilities|Select :Index (Math|Random|RandomIntegerinRange 0 1) :Option%200 (Variables|Default|GetLevel1_NPC) :Option%201 (Variables|Default|GetLevel2_NPC) :Option%202 (Variables|Default|GetLevel3_NPC) :Option%203 (Variables|Default|GetLevel4NPC) :Option%204 (Variables|Default|GetLevel5_NPC) :Option%205 0) :!label _label)
  ;[1 1 1] Random Rotation
  (Transformation|SetActorRotation (Math|Rotator|MakeRotator 0.0 0.0 (Math|Random|RandomFloatinRange 0.0 3.6e+02)))
  (Utilities|FlowControl|Delay (Math|Random|RandomFloatinRange 1e+01 2e+01))
  (goto _label))

(fn ConstructionScript)