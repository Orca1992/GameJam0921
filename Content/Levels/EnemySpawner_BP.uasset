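; EnemySpawner_BP is a level actor that spawns NPCs at random delay intervals, starting on BeginPlay or through ActivateSpawner.
; It can gather SpawnPoint_Bp actors by matching ID, but uses one only when exactly one matches, otherwise spawning at its own transform.
; A delay loop repeats endlessly when Count is -1, or counts down and then destroys the spawner.
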(event Custom|StartSpawning
  (Utilities|FlowControl|Delay (Math|Random|RandomFloatinRange (Variables|Default|GetSpawnDelay_Min) (Variables|Default|GetSpawnDelay_Max)) :!label _label)
  (if (Variables|Default|GetUserSpawnPoints)
    (if (== (Utilities|Array|Length (Variables|Default|GetSpawnPoints)) 1)
      (Variables|Default|SetSpawnLocation (Transformation|GetActorTransform (Utilities|Array|Get(acopy) (Variables|Default|GetSpawnPoints))))
      (else
        (Variables|Default|SetSpawnLocation (Transformation|GetActorTransform))))
    (else
      (Variables|Default|SetSpawnLocation (Transformation|GetActorTransform))))
  (Game|SpawnActorfromClass "/Game/AI/NPC/NPC.NPC_C" (Math|Transform|MakeTransform (+ (.location (Variables|Default|GetSpawnLocation)) "0, 0,3.000000") (.rotation (Variables|Default|GetSpawnLocation))) "Undefined" 0 0)
  (if (== (Variables|Default|GetCount) -1)
    (goto _label)
    (else
      (Variables|Default|SetCount (- (Variables|Default|GetCount) 1))
      (if (> (Variables|Default|GetCount) 0)
        (goto _label)
        (else
          (Utilities|FlowControl|Delay 0.2)
          (Actor|DestroyActor))))))

(event Custom|ActivateSpawner
  (CallFunction|StartSpawning))

(event EventBeginPlay
  (Utilities|FlowControl|Sequence
    (:then_0
      (if (Variables|Default|GetUserSpawnPoints)
        (bind _outactors (Actor|GetAllActorsOfClass "/Game/Levels/SpawnPoint_Bp.SpawnPoint_Bp_C"))
        (for _array_element _outactors
          (if (Utilities|Enum|Equal(Enum) (Variables|/Game/Levels/SpawnPoint_Bp.SpawnPoint_Bp_C|GetSpawnpoint_ID _array_element) (Variables|Default|GetSpawnPoints_ID))
            (Utilities|Array|AddUnique (Variables|Default|GetSpawnPoints) _array_element)))))
    (:then_1
      (if (Variables|Default|GetStartActive)
        (CallFunction|StartSpawning)))))

(fn ConstructionScript)